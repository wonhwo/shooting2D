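; BP_Enemy is an enemy actor that flies in a straight line and ends the game when it overlaps the player.
; On spawn, a random roll against RateToPlayer aims it at the player's position at that moment, otherwise along its forward vector.
; Tick moves it along that fixed direction by Speed and delta time, without sweep.
; Overlapping BP_Player destroys both actors, pauses the game, and shows WBP_GAMEOVER with cursor and UI-only input.
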(event EventBeginPlay
  ;[0.15 0.15 0.15 0.5] 스폰시 30% 확률로 플레이어를 향해서 이동 다른 경우는 앞으로 이동
  (if (< (Math|Random|RandomIntegerinRange 0 9) (Variables|Default|GetRateToPlayer))
    (Utilities|IsValid (Game|Player|GetPlayerPawn 0)
      (:Is%20Valid
        (Variables|Default|SetDirection (Math|Vector|Normalize (- (Transformation|GetActorLocation (Game|Player|GetPlayerPawn 0)) (Transformation|GetActorLocation))))))
    (else
      (Variables|Default|SetDirection (Transformation|GetActorForwardVector)))))

(event Collision|EventActorBeginOverlap
  (params (OtherActor :type Actor%20Object%20Reference))
  (bind _returnvalue (Game|GetPlayerController 0))
  ;[0.15 0.15 0.15 0.5] 플레이어 파괴시 게임오버 처리
  (bind _asbp_player (Utilities|Casting|CastToBP_Player OtherActor))
  (Actor|DestroyActor _asbp_player)
  (Actor|DestroyActor)
  (Game|SetGamePaused true)
  (bind _returnvalue_2 (UserInterface|CreateWidget "/Game/LHW/UI/WBP_GAMEOVER.WBP_GAMEOVER_C"))
  (UserInterface|Viewport|AddtoViewport _returnvalue_2 0)
  ;[0.15 0.15 0.15 0.5] 게임오버 이후 커서가 보이고 ui가 입력 받도록 하기
  (Variables|/Script/Engine.PlayerController|SetbShowMouseCursor _returnvalue true)
  (Input|SetInputModeUIOnly _returnvalue 0 "DoNotLock" true))

(event EventTick
  (params (DeltaSeconds :type Float%20%28single-precision%29))
  (Transformation|SetActorLocation (+ (Transformation|GetActorLocation) (* (Variables|Default|GetDirection) (Variables|Default|GetSpeed) (Utilities|Time|GetWorldDeltaSeconds))) false false))

(fn ConstructionScript)