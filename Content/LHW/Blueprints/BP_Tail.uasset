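; BP_Tail is an actor that follows a target, defaulting to player pawn 0 at BeginPlay when no Target is set.
; Each Tick, while the player pawn is valid, it passes the normalized direction toward Target to Translate.
; Translate moves it at Speed scaled by delta time, without sweep, so movement ignores collision.
; Tick validates the player pawn rather than Target itself.
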(event EventBeginPlay
  (Utilities|IsValid (Variables|Default|GetTarget)
    (:Is%20Not%20Valid
      (Variables|Default|SetTarget (Game|Player|GetPlayerPawn 0)))))

(event Collision|EventActorBeginOverlap
  (params (OtherActor :type Actor%20Object%20Reference)))

(event EventTick
  (params (DeltaSeconds :type Float%20%28single-precision%29))
  (Utilities|IsValid (Game|Player|GetPlayerPawn 0)
    (:Is%20Valid
      (CallFunction|Translate (Math|Vector|Normalize (- (Transformation|GetActorLocation (Variables|Default|GetTarget)) (Transformation|GetActorLocation))) (Variables|Default|Getspeed) DeltaSeconds))))

(fn ConstructionScript)

(fn Translate
  (params (Direction :type Vector) (Speed :type Float%20%28double-precision%29) (DeltaSecond :type Float%20%28double-precision%29))
  (Transformation|SetActorLocation (+ (Transformation|GetActorLocation) (* Direction Speed DeltaSecond)) false false))